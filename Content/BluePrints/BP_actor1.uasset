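; BP_actor1 is an actor that presents a question with three answers when the player walks into its trigger box.
; On BeginPlay it creates a WBP_Widget from its question and answer text variables and assigns it to its Widget component.
; When the player character overlaps the Box, it shows the widget, switches BP_ThirdPersonCharacter to Swimming movement and shows the mouse cursor.
; Both overlap branches print debug text, and nothing here reverses these changes.
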(event `self.ReceiveBeginPlay`
  (bind _returnvalue (`|CreateWidget` "/Game/BluePrints/WBP_Widget.WBP_Widget_C" null (`self.Question Text`) (`self.Answer 1text`) (`self.Answer 2text`) (`self.Answer 3text`)))
  (bind _output_get (set `self.WBP_Widget` _returnvalue))
  (`WidgetComponent.SetWidget` (`self.Widget`) _output_get))

(event `self.Box.OnComponentBeginOverlap`
  (params (OverlappedComponent :type "PrimitiveComponent Object Reference") (OtherActor :type "Actor Object Reference") (OtherComp :type "PrimitiveComponent Object Reference") (OtherBodyIndex :type Integer) (bFromSweep :type Boolean) (SweepResult :type "HitResult Structure (by ref)"))
  (bind _returnvalue (`GameplayStatics.GetPlayerCharacter` 0))
  (if (== OtherActor _returnvalue)
    (`KismetSystemLibrary.PrintText` "massou")
    (`SceneComponent.SetVisibility` (`self.Widget`) true false)
    (bind _asbp_third_person_character (cast `/Game/ThirdPerson/Blueprints/BP_ThirdPersonCharacter` _returnvalue))
    (`CharacterMovementComponent.SetMovementMode` (`Character.CharacterMovement` _asbp_third_person_character) "MOVE_Swimming" 0)
    (set `PlayerController.bShowMouseCursor` true (`GameplayStatics.GetPlayerController` 0))
    (else
      (`KismetSystemLibrary.PrintText` "ma massouch"))))

(fn `UserConstructionScript`)